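; Behavior tree task that makes the cat enemy deal damage to players within its attack range.
; It casts the blackboard self object to BP_Cat and gathers pawns overlapping that cat's DamageBox.
; Each pawn implementing the player interface takes the configured damage amount, then the task finishes with success.
; A failed cast of the self object ends the logic without calling FinishExecute.
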(event `self.ReceiveExecuteAI`
  (params (OwnerController :type "AIController Object Reference") (ControlledPawn :type "Pawn Object Reference"))
  (bind _asbp_cat (cast `/Game/GameContent/Frazier/EnemyCharacters/Cat/Blueprints/BP_Cat` (`BTFunctionLibrary.GetBlackboardValueAsObject` (`self.KeySelfObject`))))
  (bind _output_get (set `self.As BP Cat` _asbp_cat))
  (for _array_element (`PrimitiveComponent.GetOverlappingActors` (`/Game/GameContent/Frazier/EnemyCharacters/Cat/Blueprints/BP_Cat.DamageBox` _output_get) "/Script/Engine.Pawn")
    (bind _asif_player (cast `/Game/GameContent/Frazier/Player/IF_Player` _array_element))
    (`/Game/GameContent/Frazier/Player/IF_Player.TakeDamage` _asif_player (`self.DamageAmount`)))
  (`self.FinishExecute` true))