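; A behavior tree service that keeps a blackboard key pointed at the nearest enemy around the AI-controlled pawn.
; Each tick it sphere-overlaps pawns within a configurable radius, keeps those implementing the IF_Enemy interface, and selects the closest by distance.
; It writes that actor to the closest-enemy key, or clears the key when no enemy is in range.
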(event `self.ReceiveTickAI`
  (params (OwnerController :type "AIController Object Reference") (ControlledPawn :type "Pawn Object Reference") (DeltaSeconds :type "Float (single-precision)"))
  (bind _returnvalue (`KismetMathLibrary.Vector_Distance` (`Actor.K2_GetActorLocation` (`self.Controlled Pawn`)) (`Actor.K2_GetActorLocation` (`self.Array Element`))))
  (bind _output_get (set `self.Controlled Pawn` ControlledPawn))
  (bind _outactors (`KismetSystemLibrary.SphereOverlapActors` (`Actor.K2_GetActorLocation` _output_get) (`self.Sphere Radius`) (`|MakeArray` "ObjectTypeQuery3" :!type "EObjectTypeQuery Enum")))
  (set `self.HasPlayerInRadius` false)
  (set `self.ActorLocation` 10000000.0)
  (for _array_element _outactors
    (bind _output_get_2 (set `self.Array Element` _array_element))
    (cast `/Game/GameContent/Frazier/EnemyCharacters/IF_Enemy` _output_get_2)
    (set `self.HasPlayerInRadius` true)
    (if (< _returnvalue (`self.ActorLocation`))
      (set `self.ActorLocation` _returnvalue)
      (set `self.Enemy` (`self.Array Element`))))
  (if (`self.HasPlayerInRadius`)
    (`BTFunctionLibrary.SetBlackboardValueAsObject` (`self.KeyClosestEnemy`) (`self.Enemy`))
    (else
      (`BTFunctionLibrary.ClearBlackboardValue` (`self.KeyClosestEnemy`)))))