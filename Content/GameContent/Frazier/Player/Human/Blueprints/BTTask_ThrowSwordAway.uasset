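; Behavior tree task that makes the human AI character throw away its sword.
; On execute it gets the BP_Human from the blackboard self object and detaches its Sword actor in world space.
; It switches the sword mesh to a physics body with simulation enabled, so no impulse is applied.
; It then sets the thrown-sword blackboard flag and finishes successfully.
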(event `self.ReceiveExecuteAI`
  (params (OwnerController :type "AIController Object Reference") (ControlledPawn :type "Pawn Object Reference"))
  (bind _swordmesh (`/Game/GameContent/Frazier/Player/Human/Sword/BP_Sword.SwordMesh` (`self.Sword`)))
  (bind _asbp_human (cast `/Game/GameContent/Frazier/Player/Human/Blueprints/BP_Human` (`BTFunctionLibrary.GetBlackboardValueAsObject` (`self.KeySelfObject`))))
  (bind _output_get (set `self.Sword` (`/Game/GameContent/Frazier/Player/Human/Blueprints/BP_Human.Sword` _asbp_human)))
  (`Actor.K2_DetachFromActor` _output_get "KeepWorld" "KeepWorld" "KeepWorld")
  (`PrimitiveComponent.SetCollisionObjectType` _swordmesh "ECC_PhysicsBody")
  (`PrimitiveComponent.SetSimulatePhysics` _swordmesh true)
  (`BTFunctionLibrary.SetBlackboardValueAsBool` (`self.KeyThrownSword`) true)
  (`self.FinishExecute` true))