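; BP_Human is the human player actor, with health and a sword.
; On BeginPlay it fills health to maximum, then spawns a BP_Sword and attaches it to the mesh's right palm socket.
; A TakeDamage event subtracts from current health.
; Tick polls health and destroys both the sword and the human once it reaches zero or below.
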(event `self.ReceiveBeginPlay`
  (`|ExecutionSequence`
    (:`then_0`
      (set `self.CurrentHealth` (`self.MaxHealth`)))
    (:`then_1`
      (bind _returnvalue (`|SpawnActorFromClass` "/Game/GameContent/Frazier/Player/Human/Sword/BP_Sword.BP_Sword_C" (`KismetMathLibrary.MakeTransform` (0.0 0.0 0.0)) "AlwaysSpawn" "OverrideRootScale" null null))
      (bind _output_get (set `self.Sword` _returnvalue))
      (`self.K2_AttachToComponent` _output_get (`self.Mesh`) "Palm-R" "SnapToTarget" "SnapToTarget" "KeepWorld" true))))

(event `/Game/GameContent/Frazier/Player/IF_Player.TakeDamage`
  (params (Amount :type "Float (double-precision)"))
  (set `self.CurrentHealth` (- (`self.CurrentHealth`) Amount)))

(event `self.ReceiveTick`
  (params (DeltaSeconds :type "Float (single-precision)"))
  ;[1 1 1] Die when health == 0
  (if (<= (`self.CurrentHealth`) 0.0)
    (`self.K2_DestroyActor` (`self.Sword`))
    (`self.K2_DestroyActor`)))

(fn `UserConstructionScript`)