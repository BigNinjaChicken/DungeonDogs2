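; Behavior Tree task that picks a location for an AI pawn to run to, away from its closest enemy.
; It reads both pawns from the Blackboard and extends the enemy-to-self offset on X and Y by a distance multiplier, keeping the pawn's own height.
; A navigation raycast toward that point supplies the hit location, which it writes to the run-location key before finishing successfully.
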(event `self.ReceiveExecuteAI`
  (params (OwnerController :type "AIController Object Reference") (ControlledPawn :type "Pawn Object Reference"))
  (bind _distancemultiplier (`self.DistanceMultiplier`))
  (bind _aspawn (cast `Pawn` (`BTFunctionLibrary.GetBlackboardValueAsObject` (`self.KeySelfObject`))))
  (bind _aspawn_2 (cast `Pawn` (`BTFunctionLibrary.GetBlackboardValueAsObject` (`self.KeyClosestEnemy`))))
  (bind (_returnvalue_x _returnvalue_y) (`KismetMathLibrary.BreakVector` (`Actor.K2_GetActorLocation` _aspawn_2)))
  (bind (_returnvalue_x_2 _returnvalue_y_2 _returnvalue_z) (`KismetMathLibrary.BreakVector` (`Actor.K2_GetActorLocation` _aspawn)))
  (bind _hitlocation (`NavigationSystemV1.NavigationRaycast` (`Actor.K2_GetActorLocation` _aspawn) (`KismetMathLibrary.MakeVector` (+ _returnvalue_x (* (- _returnvalue_x_2 _returnvalue_x) _distancemultiplier)) (+ _returnvalue_y (* (- _returnvalue_y_2 _returnvalue_y) _distancemultiplier)) _returnvalue_z) null null))
  (`BTFunctionLibrary.SetBlackboardValueAsVector` (`self.RunLocationKey`) _hitlocation)
  (`self.FinishExecute` true))