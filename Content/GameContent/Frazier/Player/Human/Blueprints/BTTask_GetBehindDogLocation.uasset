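; Behavior Tree task for the human AI that computes a follow location relative to the dog, named for a spot behind it.
; It reads the dog from the blackboard, offsets its location along its forward vector by FollowDistance, and writes the result to the follow-location key.
; The offset is added, so the sign of FollowDistance decides front or back.
; The task fails if the blackboard object is not a BP_Dog.
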(event `self.ReceiveExecuteAI`
  (params (OwnerController :type "AIController Object Reference") (ControlledPawn :type "Pawn Object Reference"))
  (bind _asbp_dog (cast `/Game/GameContent/Frazier/Player/Dog/BP_Dog` (`BTFunctionLibrary.GetBlackboardValueAsObject` (`self.KeyDogObject`)))
    (:`then`
      (`BTFunctionLibrary.SetBlackboardValueAsVector` (`self.KeyFollowLocation`) (+ (* (`Actor.GetActorForwardVector` _asbp_dog) (`self.FollowDistance`)) (`Actor.K2_GetActorLocation` _asbp_dog)))
      (`self.FinishExecute` true))
    (:`CastFailed`
      (`self.FinishExecute` false))))