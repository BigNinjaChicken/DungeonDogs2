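; Behavior tree task that makes a human AI character attack enemies in range.
; It reads the BP_Human from the blackboard and loops over pawns overlapping its DamageBox.
; Through the IF_Enemy interface, a blocking target sets the lost-sword blackboard flag, while any other target takes damage.
; The task then finishes successfully.
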(event `self.ReceiveExecuteAI`
  (params (OwnerController :type "AIController Object Reference") (ControlledPawn :type "Pawn Object Reference"))
  (bind _asbp_human (cast `/Game/GameContent/Frazier/Player/Human/Blueprints/BP_Human` (`BTFunctionLibrary.GetBlackboardValueAsObject` (`self.KeySelfObject`))))
  (bind _output_get (set `self.AsBP_Human` _asbp_human))
  (for _array_element (`PrimitiveComponent.GetOverlappingActors` (`/Game/GameContent/Frazier/Player/Human/Blueprints/BP_Human.DamageBox` _output_get) "/Script/Engine.Pawn")
    (bind _asif_enemy (cast `/Game/GameContent/Frazier/EnemyCharacters/IF_Enemy` _array_element))
    (bind _return (`/Game/GameContent/Frazier/EnemyCharacters/IF_Enemy.IsBlocking` _asif_enemy))
    (if _return
      (`BTFunctionLibrary.SetBlackboardValueAsBool` (`self.KeyLostSword`) true)
      (else
        (`/Game/GameContent/Frazier/EnemyCharacters/IF_Enemy.TakeDamage` _asif_enemy (`self.DamageAmount`)))))
  (`self.FinishExecute` true))