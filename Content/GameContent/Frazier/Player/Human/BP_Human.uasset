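; BP_Human is the human player actor, holding a simple health pool that removes it from play when depleted.
; BeginPlay fills current health from max health, and a TakeDamage event subtracts the incoming amount.
; Tick polls health every frame and destroys the actor once it reaches zero or below, rather than checking when damage lands.
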(event `self.ReceiveBeginPlay`
  (set `self.CurrentHealth` (`self.MaxHealth`)))

(event `/Game/GameContent/Frazier/Player/IF_Player.TakeDamage`
  (params (Amount :type "Float (double-precision)"))
  (set `self.CurrentHealth` (- (`self.CurrentHealth`) Amount)))

(event `self.ReceiveTick`
  (params (DeltaSeconds :type "Float (single-precision)"))
  ;[1 1 1] Die when health == 0
  (if (<= (`self.CurrentHealth`) 0.0)
    (`self.K2_DestroyActor`)))

(fn `UserConstructionScript`)